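; EpicCharacter is a character Blueprint that prints debug measurements of its jumps.
; Jump start records time and position, Tick detects the apex when vertical velocity turns from positive to negative, and landing reports total airtime and distance.
; A separate Hold macro, unused in the event graph shown, tells a tap from a hold using a retriggerable delay and two gates.
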(event EventOnJumped
  (Variables|Default|SetJumpStartTime (Utilities|Time|GetTimeSeconds))
  (Variables|Default|SetStartPosition (Transformation|GetActorLocation))
  (Development|PrintString (Utilities|String|ToString(Vector) (Transformation|GetActorLocation)) true true "(R=1.000000,G=0.603922,B=0.058824,A=1.000000)"))

(event EventOnLanded
  (params (Hit :type Hit%20Result%20Structure%20%28by%20ref%29))
  (Development|PrintString "JumpTime:" true true "(R=0.000000,G=0.660000,B=1.000000,A=1.000000)" 1e+01)
  (Development|PrintString (Utilities|String|ToString(Float) (- (Utilities|Time|GetTimeSeconds) (Variables|Default|GetJumpStartTime))) true true "(R=0.000000,G=0.660000,B=1.000000,A=1.000000)" 1e+01)
  (Development|PrintString "JumpDistance:" true true "(R=1.000000,G=0.603922,B=0.058824,A=1.000000)" 1e+01)
  (Development|PrintString (Utilities|String|ToString(Float) (Math|Vector|VectorLength (- (Variables|Default|GetStartPosition) (Transformation|GetActorLocation)))) true true "(R=1.000000,G=0.603922,B=0.058824,A=1.000000)" 1e+01))

(event EventTick
  (params (DeltaSeconds :type Float%20%28single-precision%29))
  (if (and (> (.z (Variables|Default|GetLastVelocity)) 0.0) (< (.z (Transformation|GetVelocity)) 0.0))
    (Development|PrintString "ApexTime:" true true "(R=0.213908,G=1.000000,B=0.147295,A=1.000000)" 1e+01)
    (Development|PrintString (Utilities|String|ToString(Float) (- (Utilities|Time|GetTimeSeconds) (Variables|Default|GetJumpStartTime))) true true "(R=0.212231,G=1.000000,B=0.147027,A=1.000000)" 1e+01))
  (Variables|Default|SetLastVelocity (Transformation|GetVelocity)))

(fn ConstructionScript)